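; A speed-boost terrain piece that makes the first-person player walk faster while overlapping its mesh.
; On begin overlap it saves the character's current max walk speed and raises it by half.
; On end overlap it restores the saved speed.
; Both events print debug messages, including one when the overlapping actor is not the player.
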(event `self.StaticMesh1.OnComponentBeginOverlap`
  (params (OverlappedComponent :type "PrimitiveComponent Object Reference") (OtherActor :type "Actor Object Reference") (OtherComp :type "PrimitiveComponent Object Reference") (OtherBodyIndex :type Integer) (bFromSweep :type Boolean) (SweepResult :type "HitResult Structure (by ref)"))
  (`KismetSystemLibrary.PrintString` "Speed")
  (bind _asfirst_person_character (cast `/Game/Blueprints/Player/FirstPersonCharacter` OtherActor)
    (:`then`
      (bind _charactermovement (`Character.CharacterMovement` _asfirst_person_character))
      (bind _output_get (set `self.PlayerInitialMove` (`CharacterMovementComponent.MaxWalkSpeed` _charactermovement)))
      (set `CharacterMovementComponent.MaxWalkSpeed` (* _output_get 1.5) _charactermovement))
    (:`CastFailed`
      (`KismetSystemLibrary.PrintString` "Not player"))))

(event `self.StaticMesh1.OnComponentEndOverlap`
  (params (OverlappedComponent :type "PrimitiveComponent Object Reference") (OtherActor :type "Actor Object Reference") (OtherComp :type "PrimitiveComponent Object Reference") (OtherBodyIndex :type Integer))
  (`KismetSystemLibrary.PrintString` "No Speed")
  (bind _asfirst_person_character (cast `/Game/Blueprints/Player/FirstPersonCharacter` OtherActor)
    (:`then`
      (set `CharacterMovementComponent.MaxWalkSpeed` (`self.PlayerInitialMove`) (`Character.CharacterMovement` _asfirst_person_character)))
    (:`CastFailed`
      (`KismetSystemLibrary.PrintString` "Not player"))))

(fn `UserConstructionScript`)