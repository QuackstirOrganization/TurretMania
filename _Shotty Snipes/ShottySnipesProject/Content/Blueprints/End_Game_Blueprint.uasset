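; End-of-level goal actor that loads the next level by name when hit, once the game mode's enemy count reaches zero.
; On BeginPlay it creates a dynamic material from M_EndObject and binds to the FirstPersonGameMode's subtract-enemy event.
; When that event reports no enemies left, it sets the OpacityChange parameter to change the mesh's appearance; otherwise it prints a reminder to kill more.
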(event `self.ReceiveHit`
  (params (MyComp :type "PrimitiveComponent Object Reference") (Other :type "Actor Object Reference") (OtherComp :type "PrimitiveComponent Object Reference") (bSelfMoved :type Boolean) (HitLocation :type "Vector Structure") (HitNormal :type "Vector Structure") (NormalImpulse :type "Vector Structure") (Hit :type "HitResult Structure (by ref)"))
  (bind _asfirst_person_game_mode (cast `/Game/Blueprints/GameMode/FirstPersonGameMode` (`GameplayStatics.GetGameMode`))
    (:`then`
      (if (<= (`/Game/Blueprints/GameMode/FirstPersonGameMode.EnemyCurrentAmount` _asfirst_person_game_mode) 0)
        (`GameplayStatics.OpenLevel` (`self.Level Name`))))
    (:`CastFailed`
      (`KismetSystemLibrary.PrintString` "Next Level Failed"))))

(event `self.ReceiveBeginPlay`
  (bind _returnvalue (`PrimitiveComponent.CreateDynamicMaterialInstance` (`self.StaticMeshComponent`) 0 "/Game/Assets/Materials/M_EndObject.M_EndObject" "None"))
  (set `self.NewVar_0` _returnvalue)
  (bind _asfirst_person_game_mode (cast `/Game/Blueprints/GameMode/FirstPersonGameMode` (`GameplayStatics.GetGameMode`)))
  (add `/Game/Blueprints/GameMode/FirstPersonGameMode.Event_SubtractEnemy` _asfirst_person_game_mode (delegate `EnemyDied`)))

(event `EnemyDied`
  (params (NewParam :type Integer))
  (if (<= NewParam 0)
    (`MaterialInstanceDynamic.SetScalarParameterValue` (`self.NewVar_0`) "OpacityChange" 1.0)
    (else
      (`KismetSystemLibrary.PrintString` "Kill More Enemies"))))

(fn `UserConstructionScript`)